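; Player-controlled tank pawn that drives, aims a camera rig and fires.
; On BeginPlay it passes its barrel and turret to setter functions and its left and right tracks to the TankMovement component.
; Movement axes forward to TankMovement, while aim axes yaw an azimuth gimbal and pitch the spring arm separately.
; The Fire input calls the pawn's Fire function, defined outside these graphs.
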(event EventBeginPlay
  (Utilities|FlowControl|Sequence
    (:then_0
      (Class|TAnk|BarrelSetter (Variables|Default|GetBarrel))
      (Class|TAnk|TurretSetter (Variables|Default|GetTurret)))
    (:then_1
      (Class|TankMovementComponent|TrackSetter (Variables|Default|GetTankMovement) (Variables|Default|GetRight%20Track) (Variables|Default|GetLeft%20Track)))))

(event Input|ActionEvents|InputActionFire
  (params (Key :type Key%20Structure))
  ;[1 1 1] Fire
  (:Pressed
    (Class|TAnk|Fire)))

(event Input|AxisEvents|InputAxisAimAzimuth
  (params (AxisValue :type Float%20%28single-precision%29))
  ;[1 1 1] X Axis (Azimuth)
  (Transformation|AddLocalRotation (Variables|Default|GetAzimuth%20Gimbal) (Math|Rotator|MakeRotator 0.0 0.0 (* AxisValue 2.0)) false false))

(event Input|AxisEvents|InputAxisAimElavation
  (params (AxisValue :type Float%20%28single-precision%29))
  ;[1 1 1] Y Axis (Elevation)
  (Transformation|AddLocalRotation (Variables|Default|GetSpringArm) (Math|Rotator|MakeRotator 0.0 (* AxisValue 2.0) 0.0) false false))

(event Input|AxisEvents|InputAxisMoveForward
  (params (AxisValue :type Float%20%28single-precision%29))
  (Class|TankMovementComponent|MoveForward (Variables|Default|GetTankMovement) AxisValue))

(event Input|AxisEvents|InputAxisRotateRight
  (params (AxisValue :type Float%20%28single-precision%29))
  (Class|TankMovementComponent|RotateRight (Variables|Default|GetTankMovement) AxisValue))

(fn ConstructionScript)